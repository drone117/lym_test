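; BP_EventsManager is a test-effect manager that turns a formatted string into a show or hide lights call.
; On BeginPlay it caches all BP_TestEffect actors and splits InputString on semicolons and colons into effect name, event and speed.
; ExecuteEvent calls CallEDShowLights for "ShowLights", otherwise CallEDHideLights, passing speed and effect type.
; Its loop returns after the first actor, so only that one receives the call.
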(event `self.ReceiveBeginPlay`
  (bind (_lefts _rights) (`KismetStringLibrary.Split` (`self.InputString`) ";"))
  (bind (_lefts_2 _rights_2) (`KismetStringLibrary.Split` _rights ";"))
  (bind _outactors (`GameplayStatics.GetAllActorsOfClass` "/Game/Task03/Blueprints/BP_TestEffect.BP_TestEffect_C"))
  (set `self.TestEffectActors` _outactors)
  (`self.ExecuteEvent` (`KismetStringLibrary.Conv_StringToName` (`.RightS` (`KismetStringLibrary.Split` _lefts ":"))) (`KismetStringLibrary.Conv_StringToName` (`.RightS` (`KismetStringLibrary.Split` _lefts_2 ":"))) (`KismetStringLibrary.Conv_StringToDouble` (`.RightS` (`KismetStringLibrary.Split` _rights_2 ":")))))

(fn `ExecuteEvent`
  (params (EffectName :type Name) (Event :type Name) (Speed :type "Float (double-precision)"))
  (for _array_element (`self.TestEffectActors`)
    (if (== Event "ShowLights")
      (`/Game/Task03/Blueprints/BP_TestEffect.ED_ShowLights` _array_element Speed EffectName)
      (else
        (`/Game/Task03/Blueprints/BP_TestEffect.ED_HideLights` _array_element Speed EffectName)))
    (return)))

(fn `UserConstructionScript`)