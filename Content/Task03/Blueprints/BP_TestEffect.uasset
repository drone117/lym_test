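; BP_TestEffect is a controller actor that shows or hides two groups of lights, picked by a type string.
; On BeginPlay it caches all actors tagged Sphere and Cube, then binds handlers to its show and hide event dispatchers.
; Each handler selects the Sphere group, or Cube for any other type, and forwards the speed to every actor through interface messages.
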(event `self.ReceiveBeginPlay`
  (bind _outactors (`GameplayStatics.GetAllActorsWithTag` "Sphere"))
  (set `self.SphereLights` _outactors)
  (bind _outactors_2 (`GameplayStatics.GetAllActorsWithTag` "Cube"))
  (set `self.CubeLights` _outactors_2)
  (add `self.ED_ShowLights` (delegate `ShowLights`))
  (add `self.ED_HideLights` (delegate `HideLights`)))

(event `ShowLights` :!signature `self.ED_ShowLights`
  (params (Speed :type "Float (double-precision)") (Type :type Name))
  (if (== Type "Sphere")
    (for _array_element (`self.SphereLights`)
      (message `/Game/Task03/Blueprints/BPI_LightsInterface.ShowLightsInterface` _array_element Speed))
    (else
      (for _array_element_2 (`self.CubeLights`)
        (message `/Game/Task03/Blueprints/BPI_LightsInterface.ShowLightsInterface` _array_element_2 Speed)))))

(event `HideLights` :!signature `self.ED_HideLights`
  (params (Speed :type "Float (double-precision)") (Type :type Name))
  (if (== Type "Sphere")
    (for _array_element (`self.SphereLights`)
      (message `/Game/Task03/Blueprints/BPI_LightsInterface.HideLightsInterface` _array_element Speed))
    (else
      (for _array_element_2 (`self.CubeLights`)
        (message `/Game/Task03/Blueprints/BPI_LightsInterface.HideLightsInterface` _array_element_2 Speed)))))

(fn `UserConstructionScript`)