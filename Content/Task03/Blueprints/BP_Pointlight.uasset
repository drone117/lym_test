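; BP_Pointlight is a point light actor that fades in and out through show and hide interface events.
; It caches the light's starting intensity at BeginPlay, and a timeline lerps between zero and that value.
; Show plays the timeline from the start and hide reverses it from the end, with the caller's Speed as play rate.
; The construction script sets the light's visibility from IsOn.
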(event `self.ReceiveBeginPlay`
  (set `self.DefaultIntensity` (`LightComponentBase.Intensity` (`self.PointLight`))))

(event `/Game/Task03/Blueprints/BPI_LightsInterface.ShowLightsInterface`
  (params (Speed :type "Float (double-precision)"))
  (`TimelineComponent.SetPlayRate` (`self.TL_ShowLights`) Speed)
  (bind (_direction _intensity) (`Timeline|TL_ShowLights` :!via `PlayFromStart` :!label _label)
    (:`Update`
      (`LightComponent.SetIntensity` (`self.PointLight`) (`KismetMathLibrary.Lerp` 0.0 (`self.DefaultIntensity`) _intensity)))))

(event `/Game/Task03/Blueprints/BPI_LightsInterface.HideLightsInterface`
  (params (Speed :type "Float (double-precision)"))
  (`TimelineComponent.SetPlayRate` (`self.TL_ShowLights`) Speed)
  (goto _label :!via `ReverseFromEnd`))

(fn `UserConstructionScript`
  (`SceneComponent.SetVisibility` (`self.PointLight`) (`self.IsOn`) false))