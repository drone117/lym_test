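; BP_SphereController is an input controller that drives a BP_Sphere actor in the level from the number pad.
; On BeginPlay it finds the sphere with GetActorOfClass and stores the reference.
; NumPad 0 and 1 move the sphere up and down, while NumPad 2 and 3 raise and lower its emission, all by calling functions on BP_Sphere.
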(event `self.ReceiveBeginPlay`
  (bind _returnvalue (`GameplayStatics.GetActorOfClass` "/Game/Task01/Blueprints/BP_Sphere.BP_Sphere_C"))
  (set `self.SphereActor` _returnvalue))

(event `Key|NumPadZero`
  (params (Key :type "Key Structure"))
  (:`Pressed`
    (`/Game/Task01/Blueprints/BP_Sphere.MoveSphereUp` (`self.SphereActor`))))

(event `Key|NumPadOne`
  (params (Key :type "Key Structure"))
  (:`Pressed`
    (`/Game/Task01/Blueprints/BP_Sphere.MoveSphereDown` (`self.SphereActor`))))

(event `Key|NumPadTwo`
  (params (Key :type "Key Structure"))
  (:`Pressed`
    (`/Game/Task01/Blueprints/BP_Sphere.IncreaseEmission` (`self.SphereActor`))))

(event `Key|NumPadThree`
  (params (Key :type "Key Structure"))
  (:`Pressed`
    (`/Game/Task01/Blueprints/BP_Sphere.DecreaseEmission` (`self.SphereActor`))))

(fn `UserConstructionScript`)