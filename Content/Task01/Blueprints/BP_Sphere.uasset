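; BP_Sphere is a sphere actor that animates showing, hiding and glowing through events called on it.
; BeginPlay creates a dynamic material instance, whose Opacity and Emissive parameters are driven by timelines.
; MoveSphereUp and MoveSphereDown lerp the actor 300 units vertically while fading it in or out, with play rate set by ShowAnimPlayRate.
; IncreaseEmission raises Emissive toward MaxEmissive, and DecreaseEmission plays that timeline in reverse.
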(event `self.ReceiveBeginPlay`
  ;[1 1 1] Create dynamic material
  (bind _returnvalue (`PrimitiveComponent.CreateDynamicMaterialInstance` (`self.Sphere`) 0 "/Game/Task01/Materials/MI_SphereMaterial.MI_SphereMaterial" "None"))
  (set `self.DynamicMaterial` _returnvalue))

(event `MoveSphereUp`
  ;[1 1 1] Set current location and targets to move
  (bind _output_get (set `self.CurrectSphereLocation` (`self.K2_GetActorLocation`)))
  (set `self.TargetToMove` (`KismetMathLibrary.MakeVector` (.x _output_get) (.y _output_get) (+ (.z _output_get) 300.0)))
  (`|ExecutionSequence`
    (:`then_0`
      (`TimelineComponent.SetPlayRate` (`self.TL_ChangeOpacity`) (`self.ShowAnimPlayRate`))
      ;[1 1 1] Change opacity
      (bind (_direction _opacitytrack) (`Timeline|TL_ChangeOpacity` :`NewTime` 2.0 :!via `PlayFromStart` :!label _label)
        (:`Update`
          (`MaterialInstanceDynamic.SetScalarParameterValue` (`self.DynamicMaterial`) "Opacity" _opacitytrack))))
    (:`then_1`
      (`TimelineComponent.SetPlayRate` (`self.TL_MoveSphereUp`) (`self.ShowAnimPlayRate`))
      ;[1 1 1] Move actor up
      (bind (_direction_2 _movementtrack) (`Timeline|TL_MoveSphereUp` :!via `PlayFromStart`)
        (:`Update`
          (`self.K2_SetActorLocation` (`KismetMathLibrary.VLerp` (`self.CurrectSphereLocation`) (`self.TargetToMove`) _movementtrack)))))))

(event `MoveSphereDown`
  ;[1 1 1] Set current location and targets to move
  (bind _output_get (set `self.CurrectSphereLocation` (`self.K2_GetActorLocation`)))
  (set `self.TargetToMove` (`KismetMathLibrary.MakeVector` (.x _output_get) (.y _output_get) (+ (.z _output_get) -300.0)))
  (`|ExecutionSequence`
    (:`then_0`
      (`TimelineComponent.SetPlayRate` (`self.TL_ChangeOpacity`) (`self.ShowAnimPlayRate`))
      (goto _label :!via `ReverseFromEnd`))
    (:`then_1`
      (`TimelineComponent.SetPlayRate` (`self.TL_MoveSphereDown`) (`self.ShowAnimPlayRate`))
      ;[1 1 1] Move actor down
      (bind (_direction _movementtrack) (`Timeline|TL_MoveSphereDown` :!via `PlayFromStart`)
        (:`Update`
          (`self.K2_SetActorLocation` (`KismetMathLibrary.VLerp` (`self.CurrectSphereLocation`) (`self.TargetToMove`) _movementtrack)))))))

(event `IncreaseEmission`
  ;[1 1 1] Change emissive
  (bind (_direction _emissivetrack) (`Timeline|TL_ChangeEmission` :`NewTime` 3.0 :!via `PlayFromStart` :!label _label_2)
    (:`Update`
      (`MaterialInstanceDynamic.SetScalarParameterValue` (`self.DynamicMaterial`) "Emissive" (`KismetMathLibrary.Lerp` 0.0 (`self.MaxEmissive`) _emissivetrack)))))

(event `DecreaseEmission`
  (goto _label_2 :!via `ReverseFromEnd`))

(fn `UserConstructionScript`)