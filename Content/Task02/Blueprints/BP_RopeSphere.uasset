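; Rope-hung physics sphere that can be raised and lowered through events.
; MoveSphereUp and MoveSphereDown enable sphere physics, then play or reverse one shared timeline at the current Speed.
; The timeline drives the Cable length and the PhysicsConstraint's linear limits on all three axes together, so the visible rope and physical tether change in step.
; Separate events switch Speed between normal and double, applied on the next move call.
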(event `SetNormalSpeed`
  (set `self.Speed` 1.0))

(event `SetDoubleSpeed`
  (set `self.Speed` 2.0))

(event `MoveSphereUp`
  (bind _physicsconstraint (`self.PhysicsConstraint`))
  (`PrimitiveComponent.SetSimulatePhysics` (`self.Sphere`) true)
  (`TimelineComponent.SetPlayRate` (`self.TL_MoveSphereUp`) (`self.Speed`))
  (bind (_direction _cablelength _constraintoffset) (`Timeline|TL_MoveSphereUp` :!label _label)
    (:`Update`
      (set `CableComponent.CableLength` _cablelength (`self.Cable`))
      (`PhysicsConstraintComponent.SetLinearXLimit` _physicsconstraint "LCM_Limited" _constraintoffset)
      (`PhysicsConstraintComponent.SetLinearYLimit` _physicsconstraint "LCM_Limited" _constraintoffset)
      (`PhysicsConstraintComponent.SetLinearZLimit` _physicsconstraint "LCM_Limited" _constraintoffset))
    (:`Finished`
      (`PrimitiveComponent.SetSimulatePhysics` (`self.Sphere`) true))))

(event `MoveSphereDown`
  (`PrimitiveComponent.SetSimulatePhysics` (`self.Sphere`) true)
  (`TimelineComponent.SetPlayRate` (`self.TL_MoveSphereUp`) (`self.Speed`))
  (goto _label :!via `Reverse`))

(fn `UserConstructionScript`)