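; BP_RopeSphereController maps numpad keys to control of a rope sphere actor in the level.
; On BeginPlay it finds and caches a BP_RopeSphere through GetActorOfClass.
; Key presses then call that actor's functions to move the sphere up or down and to switch between double and normal speed, leaving the movement logic to BP_RopeSphere.
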(event `self.ReceiveBeginPlay`
  (bind _returnvalue (`GameplayStatics.GetActorOfClass` "/Game/Task02/Blueprints/BP_RopeSphere.BP_RopeSphere_C"))
  (set `self.RopeSphereActor` _returnvalue))

(event `Key|NumPadFour`
  (params (Key :type "Key Structure"))
  (:`Pressed`
    (`/Game/Task02/Blueprints/BP_RopeSphere.MoveSphereUp` (`self.RopeSphereActor`))))

(event `Key|NumPadSix`
  (params (Key :type "Key Structure"))
  (:`Pressed`
    (`/Game/Task02/Blueprints/BP_RopeSphere.MoveSphereDown` (`self.RopeSphereActor`))))

(event `Key|NumPadTwo`
  (params (Key :type "Key Structure"))
  (:`Pressed`
    (`/Game/Task02/Blueprints/BP_RopeSphere.SetDoubleSpeed` (`self.RopeSphereActor`))))

(event `Key|NumPadThree`
  (params (Key :type "Key Structure"))
  (:`Pressed`
    (`/Game/Task02/Blueprints/BP_RopeSphere.SetNormalSpeed` (`self.RopeSphereActor`))))

(fn `UserConstructionScript`)